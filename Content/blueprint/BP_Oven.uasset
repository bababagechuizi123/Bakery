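; BP_Oven is an oven that bakes one cake at a time by ID and hands back the finished item with quality scores.
; An enum state gates starting, finishing and retrieval, while a looping timer, not Tick, advances bake time and drives a progress-bar widget.
; On completion it plays a ding and randomly rolls aroma, taste and appearance within the player character's Min and Max, returned on retrieval before resetting.
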(event `self.ReceiveBeginPlay`
  (bind _returnvalue (`|CreateWidget` "/Game/blueprint/UI/BakingProgressBar.BakingProgressBar_C" (`GameplayStatics.GetPlayerController` 0)))
  (bind _output_get (set `self.烘烤进度条UI` _returnvalue))
  (`UserWidget.AddToViewport` _output_get 0)
  (`Widget.SetVisibility` _output_get "Hidden"))

(fn `UserConstructionScript`)

(fn `取出蛋糕`
  (returns (`蛋糕ID` :type Integer) (`香味` :type "Float (double-precision)") (`口感` :type "Float (double-precision)") (`外观` :type "Float (double-precision)") (`取出成功` :type Boolean))
  (bind `_烘烤进度条ui` (`self.烘烤进度条UI`))
  (if (`|EnumEquality` (`self.当前状态`) "NewEnumerator2")
    (set `self.当前状态` "NewEnumerator0")
    (set `self.当前烘烤时间` 0.0)
    (`TextBlock.SetText` (`/Game/blueprint/UI/BakingProgressBar.提示文字` `_烘烤进度条ui`) "Baking...")
    (`Widget.SetVisibility` `_烘烤进度条ui` "Hidden")
    (return (`self.当前蛋糕ID`) (`self.香味`) (`self.口感`) (`self.外观`) true)
    (else
      (return 0 0.0 0.0 0.0 false))))

(fn `开始烘烤`
  (params (`目标蛋糕ID` :type Integer))
  (returns (`是否成功` :type Boolean))
  (bind `_烘烤进度条ui` (`self.烘烤进度条UI`))
  (if (`|EnumEquality` (`self.当前状态`) "NewEnumerator0")
    (set `self.当前蛋糕ID` `目标蛋糕ID`)
    (set `self.当前状态` "NewEnumerator1")
    (set `self.当前烘烤时间` 0.0)
    (`Widget.SetVisibility` `_烘烤进度条ui` "Visible")
    (`ProgressBar.SetPercent` (`/Game/blueprint/UI/BakingProgressBar.烘烤进度条` `_烘烤进度条ui`) 0.0)
    (bind _returnvalue (`KismetSystemLibrary.K2_SetTimer` null "更新烘烤" 0.05 true))
    (set `self.烘烤计时器` _returnvalue)
    (return true)
    (else
      (return false))))

(fn `更新烘烤`
  (bind _output_get (set `self.当前烘烤时间` (+ (`self.当前烘烤时间`) 0.05)))
  (`ProgressBar.SetPercent` (`/Game/blueprint/UI/BakingProgressBar.烘烤进度条` (`self.烘烤进度条UI`)) (`KismetMathLibrary.FClamp` (/ _output_get (`self.总烘烤时间`))))
  ; 完成烘烤，清空计时器，结束循环
  (if (>= (`self.当前烘烤时间`) (`self.总烘烤时间`))
    (`KismetSystemLibrary.K2_ClearAndInvalidateTimerHandle` (`self.烘烤计时器`))
    (`self.结束烘烤`)))

(fn `结束烘烤`
  (locals (`最大值` :type "Float (double-precision)" :default 0.0) (`最小值` :type "Float (double-precision)" :default 0.0))
  (`GameplayStatics.PlaySound2D` "/Game/MUSIC+VFX/烤面包机烤箱_toaster_oven_ding__爱给网_aigei_com.烤面包机烤箱_toaster_oven_ding__爱给网_aigei_com" 1.0 1.0 0.0 null null)
  (set `self.当前状态` "NewEnumerator2")
  (`TextBlock.SetText` (`/Game/blueprint/UI/BakingProgressBar.提示文字` (`self.烘烤进度条UI`)) "The bread is ready!")
  (bind _asbp_first_person_character (cast `/Game/FirstPerson/Blueprints/BP_FirstPersonCharacter` (`GameplayStatics.GetPlayerPawn` 0)))
  ; 决定蛋糕的质量
  (bind _output_get (set `local.最小值` (`/Game/FirstPerson/Blueprints/BP_FirstPersonCharacter.Min` _asbp_first_person_character)))
  (bind _output_get_2 (set `local.最大值` (`/Game/FirstPerson/Blueprints/BP_FirstPersonCharacter.Max` _asbp_first_person_character)))
  (set `self.香味` (`KismetMathLibrary.RandomFloatInRange` _output_get _output_get_2))
  (set `self.口感` (`KismetMathLibrary.RandomFloatInRange` _output_get _output_get_2))
  (set `self.外观` (`KismetMathLibrary.RandomFloatInRange` _output_get _output_get_2)))
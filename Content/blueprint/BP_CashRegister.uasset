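; BP_CashRegister is a checkout register that manages a queue of customers and completes their payment.
; Joining customers are added to an array, and each refresh sends every customer to a matching queue point, facing the register or the point ahead.
; Checkout acts only if the first customer is in a specific state, then removes them, plays a register sound, returns their checkout result and advances the line.
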(event `加入排队`
  (params (`新顾客` :type "/Game/blueprint/BP_Customer Object Reference"))
  (`/Engine/EditorBlueprintResources/StandardMacros.IsValid` `新顾客`
    (:`Is Valid`
      (`KismetArrayLibrary.Array_Add` (`self.当前排队顾客`) `新顾客`)
      (`self.刷新队伍`))))

(fn `UserConstructionScript`)

(fn `刷新队伍`
  (locals (`朝向目标` :type "Actor Object Reference"))
  (for (_array_element _array_index) (`self.当前排队顾客`)
    (if (== _array_index 0)
      (set `local.朝向目标` self)
      (else
        (set `local.朝向目标` (`|GetArrayItem` (`self.排队点数组`) (- _array_index 1)))))
    (`/Game/blueprint/BP_Customer.前往排队点` _array_element (`|GetArrayItem` (`self.排队点数组`) _array_index) (`local.朝向目标`))))

(fn `结账`
  (returns (`付款金额` :type Integer))
  (locals (`第一个顾客` :type "/Game/blueprint/BP_Customer Object Reference"))
  (if (> (`KismetArrayLibrary.Array_Length` (`self.当前排队顾客`)) 0)
    (bind _output_get (set `local.第一个顾客` (`|GetArrayItem` (`self.当前排队顾客`))))
    (if (`|EnumEquality` (`/Game/blueprint/BP_Customer.顾客状态` _output_get) "NewEnumerator3")
      (`KismetArrayLibrary.Array_Remove` (`self.当前排队顾客`))
      (`GameplayStatics.PlaySound2D` "/Game/MUSIC+VFX/收银机2_Cash_Register_2__爱给网_aigei_com.收银机2_Cash_Register_2__爱给网_aigei_com" 1.0 1.0 0.0 null null)
      (bind `_付款金额` (`/Game/blueprint/BP_Customer.完成结账` _output_get))
      (`self.刷新队伍`)
      (return `_付款金额`)
      (else
        (return 0)))
    (else
      (return 0))))
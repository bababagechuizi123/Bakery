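; BP_Tray is a bakery display tray that holds one cake type with its quality stats, cost and price for customers to take.
; On BeginPlay it gathers static meshes tagged "蛋糕"; restocking (补货) applies the type's mapped mesh, shows them and sets quantity to four.
; Purchase requires stock and a price, which is set outside these graphs.
; Each take hides one mesh and returns the price, clearing the tray after the last.
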(event `self.ReceiveBeginPlay`
  (set `self.蛋糕数组` (`self.GetComponentsByTag` "/Script/Engine.StaticMeshComponent" "蛋糕")))

(fn `UserConstructionScript`
  (`StaticMeshComponent.SetStaticMesh` (`self.托盘`) (`self.托盘模型`)))

(fn `是否可以购买`
  (returns (`是否可以购买` :type Boolean))
  (if (and (> (`self.数量`) 0) (> (`self.价格`) -1))
    (return true)
    (else
      (return false))))

(fn `清空托盘`
  (set `self.蛋糕ID` -1)
  (set `self.数量` 0)
  (set `self.香味` 0.0)
  (set `self.口感` 0.0)
  (set `self.外观` 0.0)
  (set `self.价格` -1)
  (for _array_element (`self.蛋糕数组`)
    (`SceneComponent.SetVisibility` _array_element false false)))

(fn `补货`
  (params (`新蛋糕种类` :type Integer) (`新香味` :type "Float (double-precision)") (`新口感` :type "Float (double-precision)") (`新外观` :type "Float (double-precision)") (`成本` :type Integer))
  (returns (`补货成功` :type Boolean))
  (set `self.蛋糕ID` `新蛋糕种类`)
  (set `self.香味` `新香味`)
  (set `self.口感` `新口感`)
  (set `self.外观` `新外观`)
  (set `self.成本` `成本`)
  (for _array_element (`self.蛋糕数组`)
    (`StaticMeshComponent.SetStaticMesh` _array_element (`|GetArrayItem` (`self.蛋糕模型映射表`) (`self.蛋糕ID`)))
    (`SceneComponent.SetVisibility` _array_element true false))
  (set `self.数量` 4)
  (return true))

(fn `顾客拿取面包`
  (returns (`拿取成功` :type Boolean) (`价格` :type Integer))
  (locals (`临时价格` :type Integer))
  (if (> (`self.数量`) 0)
    (`SceneComponent.SetVisibility` (`|GetArrayItem` (`self.蛋糕数组`) (- (`self.数量`) 1)) false false)
    (bind _output_get (set `self.数量` (- (`self.数量`) 1)))
    (if (<= _output_get 0)
      (bind _output_get_2 (set `local.临时价格` (`self.价格`)))
      (`self.清空托盘`)
      (return true _output_get_2)
      (else
        (return true (`self.价格`))))
    (else
      (return false 0))))
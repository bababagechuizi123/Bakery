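; AI customer for a bread shop that picks bread, queues at the cash register, then leaves.
; It randomizes mesh and preferences, scores BP_Tray stock by weighted quality plus sigmoid price acceptance, and walks to the best tray to buy or reject.
; AIMoveTo drives movement, while the register handles queuing and checkout.
; Probabilistic feedback turns the dominant factor into randomized sentences, shown in a bubble that timed camera traces hide when occluded.
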(event `self.ReceivePossessed`
  (params (NewController :type "Controller Object Reference"))
  (bind _asaicontroller (cast `AIController` NewController))
  (set `self.AI控制器` _asaicontroller))

(event `self.ReceiveBeginPlay`
  (`self.初始化`)
  (`KismetSystemLibrary.Delay` 0.2)
  (`self.选购面包`))

(event `前往货架`
  (bind `_选择的托盘` (`self.选择的托盘`))
  (bind `_选择的托盘_2` (`self.选择的托盘`))
  (bind `_选择的托盘_3` (`self.选择的托盘`))
  (set `self.顾客状态` "NewEnumerator0")
  (`|AIMoveTo` self (0.0 0.0 0.0) (`/Game/blueprint/BP_Tray.顾客站位` (`self.选择的托盘`)) 30.0
    (:`OnSuccess`
      (`AIController.K2_SetFocus` (`self.AI控制器`) (`self.选择的托盘`))
      (if (>= (`self.当前最高效用`) (`.最低购买效用_11_9C7F49DB43FA7A9086EC8F87595241A7` (break `/Game/blueprint/ST_Preferance` (`self.偏好`))))
        ; 拿面包
        (set `self.顾客状态` "NewEnumerator1")
        (bind (`_效用` `_价格接受度`) (`self.计算效用` (`/Game/blueprint/BP_Tray.价格` `_选择的托盘`) (`/Game/blueprint/BP_Tray.香味` `_选择的托盘`) (`/Game/blueprint/BP_Tray.口感` `_选择的托盘`) (`/Game/blueprint/BP_Tray.外观` `_选择的托盘`) (`/Game/blueprint/BP_Tray.成本` `_选择的托盘`)))
        (`KismetSystemLibrary.Delay` 3.0)
        (if (>= `_效用` (`.最低购买效用_11_9C7F49DB43FA7A9086EC8F87595241A7` (break `/Game/blueprint/ST_Preferance` (`self.偏好`))))
          (bind (`_拿取成功` `_价格`) (`/Game/blueprint/BP_Tray.顾客拿取面包` (`self.选择的托盘`)))
          (if `_拿取成功`
            (`self.开始播放拿面包动画`)
            (set `self.预付金额` `_价格`)
            (`KismetSystemLibrary.Delay` 1.3)
            (`self.停止播放拿面包动画`)
            (bind (`_反馈计划` `_反馈成功`) (`self.尝试商品反馈` true (`/Game/blueprint/BP_Tray.香味` `_选择的托盘_2`) (`/Game/blueprint/BP_Tray.口感` `_选择的托盘_2`) (`/Game/blueprint/BP_Tray.外观` `_选择的托盘_2`) `_价格接受度`))
            (`|ExecutionSequence`
              (:`then_0`
                (if `_反馈成功`
                  (bind `_反馈文本` (`self.生成商品反馈文本` `_反馈计划` (`|GetArrayItem` (`self.面包名称映射表`) (`/Game/blueprint/BP_Tray.蛋糕ID` `_选择的托盘_2`))))
                  (`self.反馈` `_反馈文本`)))
              (:`then_1`
                (`self.前往收银台`)))
            (else
              (`self.选购面包`)
              (`self.反馈` "It's already sold out?")))
          (else
            (`self.选购面包`)
            (`self.反馈` "I don't want it anymore")))
        (else
          ; 不买，只评价
          (`KismetSystemLibrary.Delay` 2.0)
          (if (> (`/Game/blueprint/BP_Tray.数量` (`self.选择的托盘`)) 0)
            (bind (`_反馈计划_2` `_反馈成功_2`) (`self.尝试商品反馈` false (`/Game/blueprint/BP_Tray.香味` `_选择的托盘_3`) (`/Game/blueprint/BP_Tray.口感` `_选择的托盘_3`) (`/Game/blueprint/BP_Tray.外观` `_选择的托盘_3`) (`self.最高价格接受度`)))
            (`|ExecutionSequence`
              (:`then_0`
                (if `_反馈成功_2`
                  (bind `_反馈文本_2` (`self.生成商品反馈文本` `_反馈计划_2` (`|GetArrayItem` (`self.面包名称映射表`) (`/Game/blueprint/BP_Tray.蛋糕ID` `_选择的托盘_3`))))
                  (`self.反馈` `_反馈文本_2`)))
              (:`then_1`
                (`self.离开店铺`)))
            (else
              (`self.反馈` "It's already sold out?")
              (`self.离开店铺`))))))))

(event `前往收银台`
  (set `self.顾客状态` "NewEnumerator2")
  (`/Game/blueprint/BP_CashRegister.加入排队` (`self.收银机引用`) self))

(event `前往排队点`
  (params (`排队点` :type "TargetPoint Object Reference") (`朝向目标` :type "Actor Object Reference"))
  (set `self.顾客状态` "NewEnumerator2")
  (`AIController.K2_ClearFocus` (`self.AI控制器`))
  (`|AIMoveTo` self (0.0 0.0 0.0) `排队点` 10.0 true
    (:`OnSuccess`
      (`AIController.K2_SetFocus` (`self.AI控制器`) `朝向目标`)
      (set `self.顾客状态` "NewEnumerator3"))))

(event `反馈`
  (params (`反馈文本` :type Text))
  ; 反馈
  (if (not (`self.正在显示反馈`))
    (`self.显示反馈` `反馈文本`)
    (`KismetSystemLibrary.Delay` 5.0)
    (`self.关闭反馈`)))

(event `离开店铺`
  ; 离开店铺
  (set `self.顾客状态` "NewEnumerator4")
  (`AIController.K2_ClearFocus` (`self.AI控制器`))
  (bind _movementresult (`|AIMoveTo` self (0.0 0.0 0.0) (`self.门所在点`) 10.0 true)
    (:`OnSuccess`
      (`self.K2_DestroyActor`))
    (:`OnFail`
      (`KismetSystemLibrary.PrintString` "寻路失败")
      (`KismetSystemLibrary.PrintString` (`KismetStringLibrary.Conv_ByteToString` _movementresult)))))

(event `开始播放拿面包动画`
  ; 动画
  (bind _asabp_cusotmer (cast `/Game/blueprint/ABP_Cusotmer` (`SkeletalMeshComponent.GetAnimInstance` (`self.Mesh`))))
  (set `/Game/blueprint/ABP_Cusotmer.是否拿面包` true _asabp_cusotmer))

(event `停止播放拿面包动画`
  ; 动画
  (bind _asabp_cusotmer (cast `/Game/blueprint/ABP_Cusotmer` (`SkeletalMeshComponent.GetAnimInstance` (`self.Mesh`))))
  (set `/Game/blueprint/ABP_Cusotmer.是否拿面包` false _asabp_cusotmer))

(event `选购面包`
  (bind `_选择的托盘` (`self.选择的托盘`))
  ; 收集非空托盘
  (`KismetArrayLibrary.Array_Clear` (`self.可选托盘数组`))
  (set `self.当前最高效用` 0.0)
  (set `self.选择的托盘` null)
  (`AIController.K2_ClearFocus` (`self.AI控制器`))
  (bind _outactors (`GameplayStatics.GetAllActorsOfClass` "/Game/blueprint/BP_Tray.BP_Tray_C"))
  (for _array_element _outactors
    (if (`self.ActorHasTag` _array_element "托盘")
      (bind `_是否可以购买` (`/Game/blueprint/BP_Tray.是否可以购买` _array_element))
      (if `_是否可以购买`
        (`KismetArrayLibrary.Array_Add` (`self.可选托盘数组`) _array_element))))
  ; 判断店内有没有面包
  (if (> (`KismetArrayLibrary.Array_Length` (`self.可选托盘数组`)) 0)
    ; 评估最高效用
    (for _array_element_2 (`self.可选托盘数组`)
      (bind (`_效用` `_价格接受度`) (`self.计算效用` (`/Game/blueprint/BP_Tray.价格` _array_element_2) (`/Game/blueprint/BP_Tray.香味` _array_element_2) (`/Game/blueprint/BP_Tray.口感` _array_element_2) (`/Game/blueprint/BP_Tray.外观` _array_element_2) (`/Game/blueprint/BP_Tray.成本` _array_element_2)))
      (if (>= `_效用` (`self.当前最高效用`))
        (set `self.当前最高效用` `_效用`)
        (set `self.选择的托盘` _array_element_2)
        (set `self.最高价格接受度` `_价格接受度`)))
    (`/Engine/EditorBlueprintResources/StandardMacros.IsValid` `_选择的托盘`
      (:`Is Valid`
        (if (`KismetArrayLibrary.Array_IsValidIndex` (`self.面包名称映射表`) (`/Game/blueprint/BP_Tray.蛋糕ID` `_选择的托盘`))
          (`self.前往货架`)
          (else
            (`self.反馈` "There's nothing I wanna buy" :!label _label)
            (`self.离开店铺`))))
      (:`Is Not Valid`
        (goto _label)))
    (else
      ; 没有面包买
      (`self.离开店铺`)
      (`self.反馈` (select `int` (`KismetMathLibrary.RandomIntegerInRange` 0 1) :`0` "Am I too late?" :`1` "Where did the bread go?" :!type "Text")))))

(fn `UserConstructionScript`)

(fn `关闭反馈`
  (set `self.正在显示反馈` false)
  (`SceneComponent.SetVisibility` (`self.顾客气泡`) false false)
  (`KismetSystemLibrary.K2_ClearAndInvalidateTimerHandle` (`self.气泡显示timer`)))

(fn `初始化`
  ; 选取随机模型
  (`SkeletalMeshComponent.SetSkeletalMeshAsset` (`self.Mesh`) (`KismetArrayLibrary.Array_Random` (`self.顾客模型数组`)))
  (`SkeletalMeshComponent.SetAnimInstanceClass` (`self.Mesh`) "/Game/blueprint/ABP_Cusotmer.ABP_Cusotmer_C")
  (bind _returnvalue (`GameplayStatics.GetActorOfClass` "/Game/blueprint/BP_CashRegister.BP_CashRegister_C"))
  (set `self.收银机引用` _returnvalue)
  (set `self.偏好` (make `/Game/blueprint/ST_Preferance` (`KismetMathLibrary.RandomIntegerInRange` 25 100) (`KismetMathLibrary.RandomFloatInRange` 0.2 1.0) (`KismetMathLibrary.RandomFloatInRange` 0.2 1.0) (`KismetMathLibrary.RandomFloatInRange` 0.2 1.0) (`KismetMathLibrary.RandomFloatInRange` 0.15 0.75) (`KismetMathLibrary.RandomFloatInRange` 0.3 0.42) (`KismetMathLibrary.RandomFloatInRange` 0.15 0.35) (`KismetMathLibrary.RandomFloatInRange` 0.6 1.8))))

(fn `完成结账`
  (returns (`付款金额` :type Integer))
  (if (`|EnumEquality` (`self.顾客状态`) "NewEnumerator3")
    (`self.离开店铺`)
    (return (`self.预付金额`))))

(fn `尝试商品反馈`
  (params (`是否决定购买` :type Boolean) (`香味` :type "Float (double-precision)") (`口感` :type "Float (double-precision)") (`外观` :type "Float (double-precision)") (`价格接受度` :type "Float (double-precision)"))
  (returns (`反馈计划` :type "/Game/blueprint/ST_反馈计划 Structure") (`反馈成功` :type Boolean))
  (locals (`临时反馈计划` :type "/Game/blueprint/ST_反馈计划 Structure") (`是否购买` :type Boolean) (`临时香味` :type "Float (double-precision)") (`临时口感` :type "Float (double-precision)") (`临时外观` :type "Float (double-precision)") (`临时价格接受度` :type "Float (double-precision)") (`价格贡献分` :type "Float (double-precision)" :default 0.0) (`临时品质分` :type "Float (double-precision)") (`品质贡献分` :type "Float (double-precision)" :default 0.0) (`香味贡献分` :type "Float (double-precision)" :default 0.0) (`口感贡献分` :type "Float (double-precision)" :default 0.0) (`外观贡献分` :type "Float (double-precision)" :default 0.0) (`当前评价值` :type "Float (single-precision)" :default 0.0))
  (bind (`_预算` `_香味权重` `_口感权重` `_外观权重` `_价格敏感度`) (break `/Game/blueprint/ST_Preferance` (`self.偏好`)))
  (bind (`_预算_2` `_香味权重_2` `_口感权重_2` `_外观权重_2`) (break `/Game/blueprint/ST_Preferance` (`self.偏好`)))
  (bind (`_预算_3` `_香味权重_3` `_口感权重_3` `_外观权重_3` `_价格敏感度_2`) (break `/Game/blueprint/ST_Preferance` (`self.偏好`)))
  (bind (`_预算_4` `_香味权重_4` `_口感权重_4` `_外观权重_4`) (break `/Game/blueprint/ST_Preferance` (`self.偏好`)))
  (set `local.是否购买` `是否决定购买`)
  (set `local.临时香味` `香味`)
  (set `local.临时口感` `口感`)
  (set `local.临时外观` `外观`)
  (set `local.临时价格接受度` `价格接受度`)
  ; 判断能否反馈
  (if (`self.正在显示反馈`)
    (return (struct) false)
    (else
      ; 决定要不要反馈
      (if (<= (`KismetMathLibrary.RandomFloatInRange` 0.0 1.0) (`self.反馈概率`))
        ; 决定反馈态度
        (setmembers `/Game/blueprint/ST_反馈计划` :`StructRef` (`local.临时反馈计划`) :`反馈态度` (select `bool` (`local.是否购买`) :`false` "NewEnumerator1" :`true` "NewEnumerator0" :!type "/Game/blueprint/E_反馈态度 Enum"))
        ; 决定反馈维度
        (set `local.价格贡献分` (`KismetMathLibrary.SelectFloat` (* (`local.临时价格接受度`) `_价格敏感度_2`) (* (- 1.0 (`local.临时价格接受度`)) `_价格敏感度_2`) (`local.是否购买`)))
        (set `local.临时品质分` (/ (+ (* `_香味权重_2` (`local.临时香味`)) (* `_口感权重_2` (`local.临时口感`)) (* `_外观权重_2` (`local.临时外观`))) (`KismetMathLibrary.FMax` (+ `_香味权重_2` `_口感权重_2` `_外观权重_2`) 0.01)))
        (bind _output_get (set `local.品质贡献分` (`KismetMathLibrary.SelectFloat` (* (- 1.0 `_价格敏感度`) (`local.临时品质分`)) (* (- 1.0 (`local.临时品质分`)) (- 1.0 `_价格敏感度`)) (`local.是否购买`))))
        (if (>= _output_get (`local.价格贡献分`))
          (`|ExecutionSequence`
            (:`then_0`
              (bind _output_get_2 (set `local.香味贡献分` (`KismetMathLibrary.SelectFloat` (* (`local.临时香味`) `_香味权重_4`) (* `_香味权重_4` (- 1.0 (`local.临时香味`))) (`local.是否购买`)))))
            (:`then_1`
              (bind _output_get_3 (set `local.口感贡献分` (`KismetMathLibrary.SelectFloat` (* (`local.临时口感`) `_口感权重_4`) (* `_口感权重_4` (- 1.0 (`local.临时口感`))) (`local.是否购买`)))))
            (:`then_2`
              (bind _output_get_4 (set `local.外观贡献分` (`KismetMathLibrary.SelectFloat` (* (`local.临时外观`) `_外观权重_4`) (* `_外观权重_4` (- 1.0 (`local.临时外观`))) (`local.是否购买`)))))
            (:`then_3`
              (bind _indexofmaxvalue (`KismetMathLibrary.MaxOfFloatArray` (`|MakeArray` _output_get_2 _output_get_3 _output_get_4 :!type "Float (single-precision)")))
              (setmembers `/Game/blueprint/ST_反馈计划` :`StructRef` (`local.临时反馈计划`) :`反馈维度` (select `int` _indexofmaxvalue :`0` "NewEnumerator0" :`1` "NewEnumerator1" :`2` "NewEnumerator2" :!type "/Game/blueprint/E_反馈维度 Enum"))
              (set `local.当前评价值` (select `int` _indexofmaxvalue :`0` (`local.临时香味`) :`1` (`local.临时口感`) :`2` (`local.临时外观`) :!type "Float (single-precision)"))
              ; 决定品质反馈程度
              (`|ExecutionSequence`
                (:`then_0`
                  (if (`local.是否购买`)
                    (if (>= (`local.当前评价值`) 0.9)
                      (setmembers `/Game/blueprint/ST_反馈计划` :`StructRef` (`local.临时反馈计划`) :`反馈程度` "NewEnumerator2")
                      (elif (>= (`local.当前评价值`) 0.75)
                        (setmembers `/Game/blueprint/ST_反馈计划` :`StructRef` (`local.临时反馈计划`) :`反馈程度` "NewEnumerator1")
                        (else
                          (setmembers `/Game/blueprint/ST_反馈计划` :`StructRef` (`local.临时反馈计划`) :`反馈程度` "NewEnumerator0"))))
                    (elif (<= (`local.当前评价值`) 0.2)
                      (setmembers `/Game/blueprint/ST_反馈计划` :`StructRef` (`local.临时反馈计划`) :`反馈程度` "NewEnumerator2")
                      (elif (<= (`local.当前评价值`) 0.4)
                        (setmembers `/Game/blueprint/ST_反馈计划` :`StructRef` (`local.临时反馈计划`) :`反馈程度` "NewEnumerator1")
                        (else
                          (setmembers `/Game/blueprint/ST_反馈计划` :`StructRef` (`local.临时反馈计划`) :`反馈程度` "NewEnumerator0"))))))
                (:`then_1`
                  (return (`local.临时反馈计划`) true)))))
          (else
            (setmembers `/Game/blueprint/ST_反馈计划` :`StructRef` (`local.临时反馈计划`) :`反馈维度` "NewEnumerator6")
            ; 决定价格反馈程度
            (`|ExecutionSequence`
              (:`then_0`
                (if (`local.是否购买`)
                  (if (>= (`local.临时价格接受度`) 0.9)
                    (setmembers `/Game/blueprint/ST_反馈计划` :`StructRef` (`local.临时反馈计划`) :`反馈程度` "NewEnumerator2")
                    (elif (>= (`local.临时价格接受度`) 0.75)
                      (setmembers `/Game/blueprint/ST_反馈计划` :`StructRef` (`local.临时反馈计划`) :`反馈程度` "NewEnumerator1")
                      (else
                        (setmembers `/Game/blueprint/ST_反馈计划` :`StructRef` (`local.临时反馈计划`) :`反馈程度` "NewEnumerator0"))))
                  (elif (<= (`local.临时价格接受度`) 0.2)
                    (setmembers `/Game/blueprint/ST_反馈计划` :`StructRef` (`local.临时反馈计划`) :`反馈程度` "NewEnumerator2")
                    (elif (<= (`local.临时价格接受度`) 0.4)
                      (setmembers `/Game/blueprint/ST_反馈计划` :`StructRef` (`local.临时反馈计划`) :`反馈程度` "NewEnumerator1")
                      (else
                        (setmembers `/Game/blueprint/ST_反馈计划` :`StructRef` (`local.临时反馈计划`) :`反馈程度` "NewEnumerator0"))))))
              (:`then_1`
                (return (`local.临时反馈计划`) true)))))
        (else
          (return (struct) false))))))

(fn `显示反馈`
  (params (`反馈文本` :type Text))
  (set `self.正在显示反馈` true)
  (bind `_as顾客气泡` (cast `/Game/blueprint/UI/顾客气泡` (`WidgetComponent.GetUserWidgetObject` (`self.顾客气泡`))))
  (`/Game/blueprint/UI/顾客气泡.设置反馈文本` `_as顾客气泡` `反馈文本`)
  ; 射线检测
  (`KismetSystemLibrary.K2_ClearAndInvalidateTimerHandle` (`self.气泡显示timer`))
  (bind _returnvalue (`KismetSystemLibrary.K2_SetTimer` null "更新气泡显示" 0.1 true))
  (set `self.气泡显示timer` _returnvalue))

(fn `更新气泡显示`
  ; 检查是否被阻挡
  (bind (_outhit _returnvalue) (`KismetSystemLibrary.LineTraceSingle` (`PlayerCameraManager.GetCameraLocation` (`GameplayStatics.GetPlayerCameraManager` 0)) (`SceneComponent.K2_GetComponentLocation` (`self.顾客气泡`)) "TraceTypeQuery1" false (`|MakeArray` self (`GameplayStatics.GetPlayerCharacter` 0) :!type "Actor Object Reference")))
  (if _returnvalue
    (`SceneComponent.SetVisibility` (`self.顾客气泡`) false false)
    (else
      (`SceneComponent.SetVisibility` (`self.顾客气泡`) true false))))

(fn `生成商品反馈文本`
  (params (`反馈计划` :type "/Game/blueprint/ST_反馈计划 Structure") (`面包名称` :type Text))
  (returns (`反馈文本` :type Text))
  (locals (`程度词` :type Text) (`评价词` :type Text))
  (bind (`_反馈维度` `_反馈态度` `_反馈程度`) (break `/Game/blueprint/ST_反馈计划` `反馈计划`))
  (set `local.程度词` (`KismetMathLibrary.SelectText` (select `/Game/blueprint/E_反馈程度` `_反馈程度` :`NewEnumerator0` (`KismetArrayLibrary.Array_Random` (`|MakeArray` "quite" "pretty" "fairly" "surprisingly" :!type "Text")) :`NewEnumerator1` (`KismetArrayLibrary.Array_Random` (`|MakeArray` "really" "very" "genuinely" "especially" :!type "Text")) :`NewEnumerator2` (`KismetArrayLibrary.Array_Random` (`|MakeArray` "absolutely" "incredibly" "exceptionally" "amazingly" :!type "Text"))) (select `/Game/blueprint/E_反馈程度` `_反馈程度` :`NewEnumerator0` (`KismetArrayLibrary.Array_Random` (`|MakeArray` "a little" "a bit" "kind of" "slightly" :!type "Text")) :`NewEnumerator1` (`KismetArrayLibrary.Array_Random` (`|MakeArray` "pretty" "rather" "really" "noticeably" :!type "Text")) :`NewEnumerator2` (`KismetArrayLibrary.Array_Random` (`|MakeArray` "extremely" "seriously" "unbelievably" "ridiculously" :!type "Text"))) (`|EnumEquality` `_反馈态度` "NewEnumerator0")))
  (set `local.评价词` (`KismetMathLibrary.SelectText` (select `/Game/blueprint/E_反馈维度` `_反馈维度` :`NewEnumerator0` (`KismetArrayLibrary.Array_Random` (`|MakeArray` "fragrant" "fresh" "inviting" "pleasant" "wonderful" "delightful" :!type "Text")) :`NewEnumerator1` (`KismetArrayLibrary.Array_Random` (`|MakeArray` "soft" "fluffy" "crispy" "chewy" "smooth" "satisfying" :!type "Text")) :`NewEnumerator2` (`KismetArrayLibrary.Array_Random` (`|MakeArray` "beautiful" "appealing" "cute" "well-made" "delicate" "exquisite" :!type "Text")) :`NewEnumerator6` (`KismetArrayLibrary.Array_Random` (`|MakeArray` "affordable" "reasonably priced" "well-priced" "cheap" :!type "Text"))) (select `/Game/blueprint/E_反馈维度` `_反馈维度` :`NewEnumerator0` (`KismetArrayLibrary.Array_Random` (`|MakeArray` "bland" "burnt" "strange" "dull" "faint" :!type "Text")) :`NewEnumerator1` (`KismetArrayLibrary.Array_Random` (`|MakeArray` "dry" "hard" "tough" "soggy" "greasy" "rough" :!type "Text")) :`NewEnumerator2` (`KismetArrayLibrary.Array_Random` (`|MakeArray` "plain" "messy" "uneven" "unappealing" "overbaked" "poorly made" :!type "Text")) :`NewEnumerator6` (`KismetArrayLibrary.Array_Random` (`|MakeArray` "expensive" "overpriced" "pricey" :!type "Text"))) (`|EnumEquality` `_反馈态度` "NewEnumerator0")))
  (return (`|FormatText` "This {Bread} {action} {Degree} {Evaluation}" `面包名称` (select `/Game/blueprint/E_反馈维度` `_反馈维度` :`NewEnumerator0` "smells" :`NewEnumerator1` "seem like" :`NewEnumerator2` "looks" :`NewEnumerator6` "is" :!type "Text") (`local.程度词`) (`local.评价词`))))

(fn `计算效用`
  (params (`价格` :type Integer) (`香味` :type "Float (double-precision)") (`口感` :type "Float (double-precision)") (`外观` :type "Float (double-precision)") (`成本` :type Integer))
  (returns (`效用` :type "Float (double-precision)") (`价格接受度` :type "Float (double-precision)"))
  (locals (`安全权重总和` :type "Float (double-precision)") (`品质分` :type "Float (double-precision)") (`心里接受价格` :type "Float (double-precision)") (`临时价格接受度` :type "Float (double-precision)"))
  (bind (`_预算` `_香味权重` `_口感权重` `_外观权重` `_价格敏感度`) (break `/Game/blueprint/ST_Preferance` (`self.偏好`)))
  (bind (`_预算_2` `_香味权重_2` `_口感权重_2` `_外观权重_2` `_价格敏感度_2` `_最低购买效用` `_价格容忍度` `_品质溢价系数`) (break `/Game/blueprint/ST_Preferance` (`self.偏好`)))
  ; 判断是否超预算
  (if (<= `价格` `_预算`)
    (bind _output_get (set `local.安全权重总和` (`KismetMathLibrary.FMax` (+ `_香味权重` `_口感权重` `_外观权重`) 0.01)))
    (set `local.品质分` (/ (+ (* `香味` `_香味权重`) (* `口感` `_口感权重`) (* `外观` `_外观权重`)) _output_get))
    (bind _output_get_2 (set `local.心里接受价格` (`KismetMathLibrary.FMin` (`KismetMathLibrary.Conv_IntToDouble` `_预算_2`) (* `成本` (+ (* `_品质溢价系数` (`KismetMathLibrary.Square` (`local.品质分`))) 1.7)))))
    (bind _output_get_3 (set `local.临时价格接受度` (/ 1.0 (+ (`KismetMathLibrary.Exp` (/ (- `价格` _output_get_2) (`KismetMathLibrary.FMax` (* _output_get_2 `_价格容忍度`) 1.0))) 1.0))))
    (return (+ (* (`local.品质分`) (- 1.0 `_价格敏感度`)) (* (`local.临时价格接受度`) `_价格敏感度`) (`KismetMathLibrary.RandomFloatInRange` -0.03 0.03)) _output_get_3)
    (else
      (return 0.0 0.0))))
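; BP_CustomerSpawner periodically spawns BP_Customer actors at an entry point while their count in the level is below a maximum.
; After an initial delay, BeginPlay starts a looping timer on 生成顾客 (spawn customer), whose random interval is rolled only once.
; Each spawn passes the checkout and exit points to the customer, avoids colliding placements, and prints a message if it fails.
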(event `self.ReceiveBeginPlay`
  (`KismetSystemLibrary.RetriggerableDelay` 20.0)
  (`self.生成顾客`)
  (`KismetSystemLibrary.K2_SetTimer` null "生成顾客" (`KismetMathLibrary.RandomFloatInRange` 3.0 13.0) true))

(fn `UserConstructionScript`)

(fn `生成顾客`
  (bind `_入口点` (`self.入口点`))
  (bind _outactors (`GameplayStatics.GetAllActorsOfClass` "/Game/blueprint/BP_Customer.BP_Customer_C"))
  (if (< (`KismetArrayLibrary.Array_Length` _outactors) (`self.最大顾客数`))
    (bind _returnvalue (`|SpawnActorFromClass` "/Game/blueprint/BP_Customer.BP_Customer_C" (`KismetMathLibrary.MakeTransform` (+ (`self.K2_GetActorLocation` `_入口点`) (0.0 0.0 124.0)) (`self.K2_GetActorRotation` `_入口点`)) "AdjustIfPossibleButDontSpawnIfColliding" "MultiplyWithRoot" null (`self.结账点`) (`self.出口点`) null))
    (`/Engine/EditorBlueprintResources/StandardMacros.IsValid` _returnvalue
      (:`Is Not Valid`
        (`KismetSystemLibrary.PrintString` "顾客生成失败！")))))